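; Base Blueprint for LEGO-style collectible studs that add to the player's score when picked up.
; On BeginPlay it looks up its stud details in the DT_Studs data table, using its Type enum converted to a name as the row.
; When a player-controlled BP_Character_Base overlaps its sphere, it adds the stud's value through the ACScore component on PC_Character and destroys itself.
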(event OnComponentBeginOverlap(Sphere)
  (params (OverlappedComponent :type Primitive%20Component%20Object%20Reference) (OtherActor :type Actor%20Object%20Reference) (OtherComp :type Primitive%20Component%20Object%20Reference) (OtherBodyIndex :type Integer) (bFromSweep :type Boolean) (SweepResult :type Hit%20Result%20Structure%20%28by%20ref%29))
  (bind _asbp_character_base (Utilities|Casting|CastToBP_Character_Base OtherActor))
  (bind _aspc_character (Utilities|Casting|CastToPC_Character (Pawn|GetController _asbp_character_base)))
  (Default|AddScore (Variables|/Game/LEGO_Project/Core/Characters/PC_Character.PC_Character_C|GetAC_Score _aspc_character) (Utilities|Struct|BreakStruct_StudTypes (Variables|Default|GetStud%20Details)))
  (Actor|DestroyActor))

(event EventBeginPlay
  (bind _returnvalue (Utilities|GetDataTableRow "/Game/LEGO_Project/Core/Collectibles/DT_Studs.DT_Studs" (Utilities|String|StringToName (Utilities|String|EnumtoString (Variables|Default|GetType))))
    (:then
      (Variables|Default|SetStud%20Details _returnvalue))))

(fn ConstructionScript)