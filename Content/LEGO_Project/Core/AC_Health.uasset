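; AC_Health is an actor component that tracks its owner's health and handles damage.
; Init caches the GI_Lego game instance and, if the owner is a PC_Character, stores it as the player reference.
; DamageHealth subtracts damage and calls OnDeath at zero or below.
; Otherwise, for players only, it writes the remaining health to the game instance's PlayerHealth map, keyed by PlayerID.
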(event Custom|Init
  (Variables|Default|SetGameInstance (.AsGI%20Lego (Utilities|Casting|CastToGI_Lego (Game|GetGameInstance))))
  (bind _aspc_character (Utilities|Casting|CastToPC_Character (Components|GetOwner)))
  (Variables|Default|SetController _aspc_character))

(event Custom|DamageHealth
  (params (DamageValue :type Integer))
  (bind _controller (Variables|Default|GetController))
  (bind _output_get (Variables|Default|SetHealth (- (Variables|Default|GetHealth) DamageValue)))
  (if (<= _output_get 0)
    (Default|CallOnDeath)
    (else
      ;[1 1 1] Update Health if Player
      (Utilities|IsValid _controller
        (:Is%20Valid
          (Utilities|Map|Add (Variables|/Game/LEGO_Project/Core/GI_Lego.GI_Lego_C|GetPlayerHealth (Variables|Default|GetGameInstance)) (Variables|/Game/LEGO_Project/Core/Characters/PC_Character.PC_Character_C|GetPlayerID _controller) (Variables|Default|GetHealth)))))))