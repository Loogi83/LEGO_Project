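; BP_DamageBox is a damage volume that repeatedly hurts anything inside its Box.
; Overlaps add and remove AC_Health components in ActorsToDamage, looked up on the controller for Pawns and on the actor otherwise.
; Each entry immediately damages every tracked component by DamageValue and starts a looping timer at Delay intervals if none is running.
; The timer is cleared when the list empties.
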(event OnComponentBeginOverlap(Box)
  (params (OverlappedComponent :type Primitive%20Component%20Object%20Reference) (OtherActor :type Actor%20Object%20Reference) (OtherComp :type Primitive%20Component%20Object%20Reference) (OtherBodyIndex :type Integer) (bFromSweep :type Boolean) (SweepResult :type Hit%20Result%20Structure%20%28by%20ref%29))
  (bind _aspawn (Utilities|Casting|CastToPawn OtherActor)
    (:then
      (Utilities|Array|Add (Variables|Default|GetActorsToDamage) (Actor|GetComponentbyClass (Pawn|GetController _aspawn) "/Game/LEGO_Project/Core/AC_Health.AC_Health_C")))
    (:CastFailed
      (Utilities|Array|Add (Variables|Default|GetActorsToDamage) (Actor|GetComponentbyClass OtherActor "/Game/LEGO_Project/Core/AC_Health.AC_Health_C"))))
  (CallFunction|Damage)
  (if (not (Utilities|Time|IsValidTimerHandle (Variables|Default|GetDamageHandle)))
    (bind _returnvalue (Utilities|Time|SetTimerbyEvent (EventDispatchers|CreateEvent :!event Custom|Damage) (Variables|Default|GetDelay) true))
    (Variables|Default|SetDamageHandle _returnvalue)))

(event OnComponentEndOverlap(Box)
  (params (OverlappedComponent :type Primitive%20Component%20Object%20Reference) (OtherActor :type Actor%20Object%20Reference) (OtherComp :type Primitive%20Component%20Object%20Reference) (OtherBodyIndex :type Integer))
  (bind _aspawn (Utilities|Casting|CastToPawn OtherActor)
    (:then
      (Utilities|Array|RemoveItem (Variables|Default|GetActorsToDamage) (Actor|GetComponentbyClass (Pawn|GetController _aspawn) "/Game/LEGO_Project/Core/AC_Health.AC_Health_C")))
    (:CastFailed
      (Utilities|Array|RemoveItem (Variables|Default|GetActorsToDamage) (Actor|GetComponentbyClass OtherActor "/Game/LEGO_Project/Core/AC_Health.AC_Health_C"))))
  (if (Utilities|Array|IsEmpty (Variables|Default|GetActorsToDamage))
    (Utilities|Time|ClearandInvalidateTimerbyHandle (Variables|Default|GetDamageHandle))))

(event Custom|Damage
  (for _array_element (Variables|Default|GetActorsToDamage)
    (Default|DamageHealth _array_element (Variables|Default|GetDamageValue))))

(fn ConstructionScript)