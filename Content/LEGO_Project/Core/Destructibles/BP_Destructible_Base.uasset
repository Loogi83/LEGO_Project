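; Base Blueprint for destructible actors in the LEGO project, which drop studs when destroyed.
; On BeginPlay it binds to the death event of its ACHealth component.
; On death, the ACStudDrop component drops studs and the actor destroys itself.
; A debug Tick draws the current health as on-screen text at the actor every frame.
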(event Custom|OnDeath
  (Default|DropStuds (Variables|Default|GetAC_StudDrop))
  (Actor|DestroyActor))

(event EventBeginPlay
  (EventDispatchers|BindEventtoOnDeath (Variables|Default|GetAC_Health) (EventDispatchers|CreateEvent :!event Custom|OnDeath)))

(event EventTick
  (params (DeltaSeconds :type Float%20%28single-precision%29))
  ;[1 1 1] Debug Tick
  (Rendering|Debug|DrawDebugString "0, 0, 0" (Utilities|String|ToString(Integer) (Variables|/Game/LEGO_Project/Core/AC_Health.AC_Health_C|GetHealth (Variables|Default|GetAC_Health))) self "(R=1.000000,G=0.944822,B=0.000000,A=1.000000)"))

(fn ConstructionScript)