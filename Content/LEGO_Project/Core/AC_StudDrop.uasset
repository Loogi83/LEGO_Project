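; Actor component that makes its owner drop collectible LEGO studs totalling a set Quantity value.
; DropStuds walks the DT_Studs rows in reverse order, using integer division and remainder to split the amount into stud denominations.
; Each stud spawns as a BP_Stud_Base of that type at the owner's location with a limited lifespan.
; A random velocity-change impulse within an upward cone scatters the studs.
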(fn DropStuds
  (bind _returnvalue (Components|GetOwner))
  (LocalVariables|SetRemainingAmount (Variables|Default|GetQuantity))
  (bind _outrownames (DataTable|GetDataTableRowNames "/Game/LEGO_Project/Core/Collectibles/DT_Studs.DT_Studs"))
  (bind _arrayelement (Utilities|Array|ReverseforEachLoop _outrownames)
    (:LoopBody
      (bind _returnvalue_2 (Utilities|GetDataTableRow "/Game/LEGO_Project/Core/Collectibles/DT_Studs.DT_Studs" _arrayelement)
        (:then
          (if (> (/ (LocalVariables|GetRemainingAmount) (.Value (Utilities|Struct|BreakStruct_StudTypes _returnvalue_2))) 0)
            (for _index (range 1 (/ (LocalVariables|GetRemainingAmount) (.Value (Utilities|Struct|BreakStruct_StudTypes _returnvalue_2))))
              ;[1 1 1] Spawn Coin
              (bind _returnvalue_3 (Game|SpawnActorfromClass "/Game/LEGO_Project/Core/Collectibles/BP_Stud_Base.BP_Stud_Base_C" (Math|Transform|MakeTransform (Transformation|GetActorLocation _returnvalue) "0, 0, 0" "1.000000,1.000000,1.000000") "AdjustIfPossibleButAlwaysSpawn" "MultiplyWithRoot" 0 (.Type (Utilities|Struct|BreakStruct_StudTypes _returnvalue_2)) 0))
              (Actor|SetLifeSpan _returnvalue_3 (Variables|Default|GetStudLifeSpan))
              ;[1 1 1] Impulse Coin
              (Physics|AddImpulse (Variables|/Game/LEGO_Project/Core/Collectibles/BP_Stud_Base.BP_Stud_Base_C|GetSphere _returnvalue_3) (* (Math|Random|RandomUnitVectorinConeinDegrees (Transformation|GetActorUpVector _returnvalue) 45.0) (Math|Random|RandomFloatinRange 2e+02 5e+02)) "None" true))
            (LocalVariables|SetRemainingAmount (Math|Integer|%(Integer) (LocalVariables|GetRemainingAmount) (.Value (Utilities|Struct|BreakStruct_StudTypes _returnvalue_2)))) ; Remainder
          ))))))