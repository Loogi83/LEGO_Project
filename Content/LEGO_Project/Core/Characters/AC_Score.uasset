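; AC_Score is a score-tracking component on the PC_Character player controller in the Lego game.
; Init caches the Lego game instance, the game mode and the owning controller.
; AddScore accumulates points, stores the running total in the game instance's PlayerScore map under the controller's PlayerID, then has the game mode's HUD refresh that player's score.
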(event Custom|AddScore
  (params (ScoreToAdd :type Integer))
  (bind _controller (Variables|Default|GetController))
  ;[1 1 1] Add
  (Variables|Default|SetScore (+ (Variables|Default|GetScore) ScoreToAdd))
  (Utilities|IsValid _controller
    (:Is%20Valid
      (Utilities|Map|Add (Variables|/Game/LEGO_Project/Core/GI_Lego.GI_Lego_C|GetPlayerScore (Variables|Default|GetGameInstance)) (Variables|/Game/LEGO_Project/Core/Characters/PC_Character.PC_Character_C|GetPlayerID _controller) (Variables|Default|GetScore))
      (Default|UpdateScore (Variables|/Game/LEGO_Project/Core/GM_Lego.GM_Lego_C|GetGameHUD (Variables|Default|GetGameMode)) (Variables|/Game/LEGO_Project/Core/Characters/PC_Character.PC_Character_C|GetPlayerID (Variables|Default|GetController))))))

(event Custom|Init
  (Variables|Default|SetGameInstance (.AsGI%20Lego (Utilities|Casting|CastToGI_Lego (Game|GetGameInstance))))
  (bind _asgm_lego (Utilities|Casting|CastToGM_Lego (Game|GetGameMode)))
  (Variables|Default|SetGameMode _asgm_lego)
  (bind _aspc_character (Utilities|Casting|CastToPC_Character (Components|GetOwner)))
  (Variables|Default|SetController _aspc_character))